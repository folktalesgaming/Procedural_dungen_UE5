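; Procedural dungeon generator actor that builds a seeded layout from room Blueprints on BeginPlay, using a random seed when Seed is -1.
; From a start room, it spawns random rooms at random open exits, destroying and retrying any that overlap after a short delay.
; Accepted rooms add their exits to the pool until RoomCount runs out, then walls cap unused exits.
; A timeout event, not called here, can open ThirdPersonMap.
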(event Custom|Start%20Room%20Spawn
  ;[0.175 1 0.2754 1 34] Start Spawn Room
  (bind _returnvalue (Game|SpawnActorfromClass "/Game/Procedural_Dungen/Dungen_Room_Variant1_BP.Dungen_Room_Variant1_BP_C" (Transformation|GetWorldTransform (Variables|Default|GetDefaultSceneRoot)) "AlwaysSpawn" "MultiplyWithRoot" 0 0))
  (Utilities|Array|AppendArray (Variables|Default|GetExits%20List) (Components|GetChildrenComponents (Variables|/Game/Procedural_Dungen/Master_Room_BP.Master_Room_BP_C|GetExits _returnvalue) false)))

(event Custom|Spawn%20Next%20Room
  ;[0.1824 1 0.3938 1 32] Spawn Next Room
  (Variables|Default|SetSelected%20Exit%20Point (.OutItem (Utilities|Array|RandomFromStream (Variables|Default|GetExits%20List) (Variables|Default|GetSeedStream))))
  (bind _returnvalue (Game|SpawnActorfromClass (.OutItem (Utilities|Array|RandomFromStream (Variables|Default|GetRooms) (Variables|Default|GetSeedStream))) (Transformation|GetWorldTransform (Variables|Default|GetSelected%20Exit%20Point)) "AlwaysSpawn" "MultiplyWithRoot" 0 0))
  (bind _asmaster_room_bp (Utilities|Casting|CastToMaster_Room_BP _returnvalue))
  (Variables|Default|SetLatest%20Room _asmaster_room_bp)
  (Utilities|FlowControl|Delay 0.2)
  (CallFunction|RemoveLatestOverlappedRoom))

(event Custom|Check%20Overlapping%20Rooms
  ;[0.3551 1 0.3672 1 32] Check Overlapping Rooms
  (for _array_element (Components|GetChildrenComponents (Variables|/Game/Procedural_Dungen/Master_Room_BP.Master_Room_BP_C|GetOverlaps (Variables|Default|GetLatest%20Room)) false)
    (bind _asbox_collision (Utilities|Casting|CastToBoxComponent _array_element))
    (Utilities|Array|AppendArray (Variables|Default|GetOverlapping%20Rooms) (Class|PrimitiveComponent|GetOverlappingComponents _asbox_collision))))

(event Custom|Remove%20Latest%20Overlapped%20Room
  ;[0.2289 1 0.3371 1 32] Remove Latest Overlapping Room
  (CallFunction|CheckOverlappingRooms)
  (if (Utilities|Array|IsNotEmpty (Variables|Default|GetOverlapping%20Rooms))
    (Utilities|Array|Clear (Variables|Default|GetOverlapping%20Rooms))
    (Actor|DestroyActor (Variables|Default|GetLatest%20Room))
    (CallFunction|SpawnNextRoom :!label _label)
    (else
      (Utilities|Array|Clear (Variables|Default|GetOverlapping%20Rooms))
      (Variables|Default|SetRoom%20Count (- (Variables|Default|GetRoom%20Count) 1))
      (Utilities|Array|RemoveItem (Variables|Default|GetExits%20List) (Variables|Default|GetSelected%20Exit%20Point))
      (Utilities|Array|AppendArray (Variables|Default|GetExits%20List) (Components|GetChildrenComponents (Variables|/Game/Procedural_Dungen/Master_Room_BP.Master_Room_BP_C|GetExits (Variables|Default|GetLatest%20Room)) false))
      (if (> (Variables|Default|GetRoom%20Count) 0)
        (goto _label)
        (else
          (CallFunction|CloseUnusedHoles)
          (Variables|Default|SetCheckDungenComplete true)
          (Utilities|Time|ClearandInvalidateTimerbyHandle (Variables|Default|GetTimer%20Hanlder)))))))

(event Custom|Close%20unused%20holes
  ;[0.3149 1 0.2686 1 32] Closing the holes
  (for _array_element (Variables|Default|GetExits%20List)
    (Game|SpawnActorfromClass "/Game/Procedural_Dungen/Close_Wall_BP.Close_Wall_BP_C" (Transformation|GetWorldTransform _array_element) "AlwaysSpawn" "MultiplyWithRoot" 0 0)))

(event Custom|Start%20dungent%20timer
  ;[0.2541 1 0.3275 1 32] Dungen Build Timer
  (bind _returnvalue (Utilities|Time|SetTimerbyEvent (delegate Custom|Check%20Dungen%20Complete) 1.0 true))
  (Variables|Default|SetTimer%20Hanlder _returnvalue))

(event Custom|Check%20Dungen%20Complete
  ;[0.2541 1 0.3275 1 32] Dungen Build Timer
  (if (>= (Utilities|Time|GetGameTimeinSeconds) (Variables|Default|GetMaxDungenBuildTime))
    (Game|OpenLevel(byName) "ThirdPersonMap")))

(event Custom|Seed%20Setter
  ;[0.2708 1 0.446 1 32] Set Seed If -1 or Random
  (if (== (Variables|Default|GetSeed) -1)
    (Class|KismetMathLibrary|SeedRandomStream (Variables|Default|GetSeedStream))
    (else
      (Math|Random|SetRandomStreamSeed (Variables|Default|GetSeedStream) (Variables|Default|GetSeed)))))

(event EventBeginPlay
  (CallFunction|SeedSetter)
  (CallFunction|StartRoomSpawn)
  (Utilities|FlowControl|Delay 0.2)
  (CallFunction|SpawnNextRoom))

(fn ConstructionScript)